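; Pool actor that drowns and respawns the player when its Cube volume is overlapped, with joke messages about Jeff.
; Any overlap plays water audio and acts on player 0's ThirdPersonCharacter, without checking what overlapped.
; The first time sets HasDrowned, plays drowning sounds and unpossesses the player after a delay; later times only print messages.
; Both branches end, after delays, by calling RespawnPlayerL and possessing the character.
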(event OnComponentBeginOverlap(Cube)
  (params (OverlappedComponent :type Primitive%20Component%20Object%20Reference) (OtherActor :type Actor%20Object%20Reference) (OtherComp :type Primitive%20Component%20Object%20Reference) (OtherBodyIndex :type Integer) (bFromSweep :type Boolean) (SweepResult :type Hit%20Result%20Structure%20%28by%20ref%29))
  (bind _returnvalue (Game|GetPlayerController 0))
  (Audio|Components|Audio|Play (Variables|Default|GetWater) 0.0)
  (bind _asthird_person_character (Utilities|Casting|CastToThirdPersonCharacter (Game|GetPlayerCharacter 0)))
  (if (Variables|/Game/ThirdPersonBP/Blueprints/ThirdPersonCharacter.ThirdPersonCharacter_C|GethasDrowned _asthird_person_character)
    (Development|PrintString "Jeff is now blessed with the ability to breathe underwater..." true true "(R=0.889819,G=0.039548,B=1.000000,A=1.000000)" 5.0)
    (Utilities|FlowControl|Delay 5.0)
    (Development|PrintString "He also developed a habit to teleport himself out of water after a while." true true "(R=1.000000,G=0.052076,B=0.918524,A=1.000000)" 5.0)
    (else
      (Variables|/Game/ThirdPersonBP/Blueprints/ThirdPersonCharacter.ThirdPersonCharacter_C|SethasDrowned _asthird_person_character true)
      (Audio|Components|Audio|Play (Variables|Default|GetDrowning_splash_plus_bubbles) 0.0)
      (Audio|Components|Audio|Play (Variables|Default|Getdrowning_voice) 0.0)
      (Development|PrintString "Jeff forgot that he didn't know how to swim." true true "(R=0.000000,G=0.660000,B=1.000000,A=1.000000)" 5.0)
      (Utilities|FlowControl|Delay 2.0)
      (Pawn|UnPossess _returnvalue)
      (Utilities|FlowControl|Delay 4.0)))
  (Default|RespawnPlayerL _asthird_person_character)
  (Pawn|Possess _returnvalue _asthird_person_character))

(fn ConstructionScript)